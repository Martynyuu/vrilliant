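; BP_WeaponSpawner is a pickup spawner that spawns a per-instance configurable actor class at its SpawnPoint on BeginPlay and respawns it after collection.
; When a first-person character leaves the Sphere and the spawned actor is gone, it clears Active, then restores it after RespawnTime.
; Active's RepNotify drives the state, toggling the Sphere's overlap events and spawning or destroying the actor.
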(event OnComponentEndOverlap(Sphere)
  (params (OverlappedComponent :type Primitive%20Component%20Object%20Reference) (OtherActor :type Actor%20Object%20Reference) (OtherComp :type Primitive%20Component%20Object%20Reference) (OtherBodyIndex :type Integer))
  (Utilities|Casting|CastToBP_FirstPersonCharacter OtherActor)
  (Utilities|IsValid (Variables|Default|GetSpawnedActor)
    (:Is%20Not%20Valid
      (Variables|Default|SetActive false)
      (CallFunction|UpdateSpawner))))

(event Custom|UpdateSpawner
  (Utilities|FlowControl|Delay (Variables|Default|GetRespawnTime))
  (Variables|Default|SetActive true))

(event EventBeginPlay
  (Variables|/Script/Engine.PrimitiveComponent|SetbGenerateOverlapEvents (Variables|Default|GetSphere) (Variables|Default|GetActive))
  ;[1 1 1] changable spawned weapon per isntance possible
  (bind _returnvalue (Game|SpawnActorfromClass (Variables|Default|GetActorClassToSpawn) (Transformation|GetWorldTransform (Variables|Default|GetSpawnPoint)) "Undefined" "MultiplyWithRoot" 0 0))
  (Variables|Default|SetSpawnedActor _returnvalue))

(fn ConstructionScript)

(fn OnRepActive
  (bind _output_get (Variables|/Script/Engine.PrimitiveComponent|SetbGenerateOverlapEvents (Variables|Default|GetSphere) (Variables|Default|GetActive)))
  (if _output_get
    (bind _returnvalue (Game|SpawnActorfromClass (Variables|Default|GetActorClassToSpawn) (Transformation|GetWorldTransform (Variables|Default|GetSpawnPoint)) "Undefined" "MultiplyWithRoot" 0 0))
    (Variables|Default|SetSpawnedActor _returnvalue)
    (else
      (Utilities|IsValid (Variables|Default|GetSpawnedActor)
        (:Is%20Valid
          (Actor|DestroyActor (Variables|Default|GetSpawnedActor)))))))